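; BP_PewController is the player controller for PewGame that handles character death and respawn requests.
; CharacterKilled unpossesses the pawn on authority.
; The Respawn input prints a message while a pawn is still controlled, and otherwise calls RequestGameModeRespawn.
; That event, also authority-gated, casts the game mode to PewGame_GameMode and passes this controller to its Respawn function.
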(event `CharacterKilled`
  (`/Engine/EditorBlueprintResources/ActorMacros.Switch Has Authority`
    (:`Authority`
      (`self.UnPossess`))))

(event `InputAction|Respawn` :consume false
  (params (Key :type "Key Structure" :default "AnyKey"))
  (:`Pressed`
    (`/Engine/EditorBlueprintResources/StandardMacros.IsValid` (`self.K2_GetPawn` self)
      (:`Is Valid`
        (`KismetSystemLibrary.PrintString` "PC Still controlling pawn"))
      (:`Is Not Valid`
        (`self.RequestGameModeRespawn`)))))

(event `RequestGameModeRespawn`
  (bind _returnvalue (`GameplayStatics.GetGameMode`))
  (`/Engine/EditorBlueprintResources/ActorMacros.Switch Has Authority`
    (:`Authority`
      (`/Engine/EditorBlueprintResources/StandardMacros.IsValid` _returnvalue
        (:`Is Valid`
          (bind _aspew_game_game_mode (cast `/Game/PewGame/BP/GameMode/PewGame_GameMode` _returnvalue))
          (`/Engine/EditorBlueprintResources/StandardMacros.IsValid` _aspew_game_game_mode
            (:`Is Valid`
              (bind _returnvalue_2 (`self.CastToPlayerController` self))
              (`/Game/PewGame/BP/GameMode/PewGame_GameMode.Respawn` _aspew_game_game_mode _returnvalue_2))))))))

(fn `UserConstructionScript`)